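; Player controller for navigating a planetary space scene on an nDisplay screen, with movement, look and target lock input.
; BeginPlay adds the SpaceMovement context and passes the nDisplay eye and screen references to SetNDisplayReferences.
; Input forwards to Handle functions defined outside this file, except the movement-lock toggle; completing a planet quiz starts a cinematic fly-by.
; Blueprint graphs for flight, quaternion orbiting and cone-based planet highlighting remain but are disconnected.
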(event OnFlybyFinished(CinematicCamera))

(event OnAutoZoomFinished(CinematicCamera))

(event Custom|PlanetQuizCompleted
  (params (Planet :type Planet%20Base%20Object%20Reference))
  (Class|CinematicCameraComponent|StartFlyby (Variables|Default|GetCinematicCamera) Planet (Variables|Default|GetMinOrbitDistance)))

(event Input|EnhancedActionEvents|EnhancedInputActionIA_TargetLock
  (params (ActionValue :type Boolean) (ElapsedSeconds :type Float%20%28double-precision%29) (TriggeredSeconds :type Float%20%28double-precision%29) (InputAction :type Input%20Action%20Object%20Reference :default "/Game/CustomInputs/IA_TargetLock.IA_TargetLock"))
  ;[0.15 0.15 0.15 0.5] IA_TargetLock Logic
  (:Triggered
    (Class|MyPlayerController|HandleTargetLock))
  (:Started
    (Development|PrintString "IA_TARGETLOCK")))

(event Input|EnhancedActionEvents|EnhancedInputActionIA_MovementLock
  (params (ActionValue :type Boolean) (ElapsedSeconds :type Float%20%28double-precision%29) (TriggeredSeconds :type Float%20%28double-precision%29) (InputAction :type Input%20Action%20Object%20Reference :default "/Game/CustomInputs/IA_MovementLock.IA_MovementLock"))
  ;[0.15 0.15 0.15 0.5] IA_MovementLock Logic
  (:Triggered
    (Variables|Default|SetbMovementLocked (not (Variables|Default|GetbMovementLocked))))
  (:Started
    (Development|PrintString "IA_MOVEMENTLOCK")))

(event Input|EnhancedActionEvents|EnhancedInputActionIA_Move
  (params (ActionValue :type Vector%202D%20Structure) (ElapsedSeconds :type Float%20%28double-precision%29) (TriggeredSeconds :type Float%20%28double-precision%29) (InputAction :type Input%20Action%20Object%20Reference :default "/Game/CustomInputs/IA_Move.IA_Move"))
  (Class|MyPlayerController|HandleMove ActionValue ElapsedSeconds))

(event Input|EnhancedActionEvents|EnhancedInputActionIA_CameraLook
  (params (ActionValue :type Vector%202D%20Structure) (ElapsedSeconds :type Float%20%28double-precision%29) (TriggeredSeconds :type Float%20%28double-precision%29) (InputAction :type Input%20Action%20Object%20Reference :default "/Game/CustomInputs/IA_CameraLook.IA_CameraLook"))
  (Class|MyPlayerController|HandleCameraLook ActionValue ElapsedSeconds))

(event EventBeginPlay
  (Input|AddMappingContext (PlayerController|LocalPlayerSubsystems|GetEnhancedInputLocalPlayerSubsystem) "/Game/CustomInputs/SpaceMovement.SpaceMovement" 0 "(bIgnoreAllPressedKeysUntilRelease=True,bForceImmediately=False,bNotifyUserSettings=False)")
  (bind _returnvalue (Actor|GetActorOfClass "/Game/Blueprints/NDC_Basic.NDC_Basic_C"))
  (bind _ndisplayxform (Default|GetScreenTransform _returnvalue))
  (bind _ndisplaytransform (Default|GetEyeTransform _returnvalue))
  (Class|MyPlayerController|SetNDisplayReferences _ndisplaytransform _ndisplayxform (Variables|/Game/Blueprints/NDC_Basic.NDC_Basic_C|GetnDisplayScreen _returnvalue)))

(event EventTick
  (params (DeltaSeconds :type Float%20%28single-precision%29)))

(event EventPossess
  (params (PossessedPawn :type Pawn%20Object%20Reference)))

(fn ConstructionScript)