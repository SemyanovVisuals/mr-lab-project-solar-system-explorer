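; Planet actor with a world-space quiz panel that shows a question and answer choices for that planet.
; On BeginPlay it hides the panel, then uses its parent component's name as the DT_Quiz row key to fill WBP_PlanetQuizUI.
; Tick turns the pivot and panel toward the player pawn.
; Functions expose panel visibility and forward answer-button selection to the widget.
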(event EventBeginPlay
  ;[0.15 0.15 0.15 0.5] Quiz UI: reveal UI Panel
  (Rendering|SetVisibility (Variables|Default|GetQuizUI) false false)
  ;[0.15 0.15 0.15 0.5] Quiz UI: Populate quiz entries
  (Variables|Default|SetPlanetType (Utilities|GetObjectName (Class|Actor|GetParentComponent)))
  (CallFunction|PopulateQuiz))

(event Collision|EventActorBeginOverlap
  (params (OtherActor :type Actor%20Object%20Reference)))

(event EventTick
  (params (DeltaSeconds :type Float%20%28single-precision%29))
  (bind _quizui (Variables|Default|GetQuizUI))
  (bind _uipivot (Variables|Default|GetUIPivot))
  ;[0.15 0.15 0.15 0.5] Quiz UI: Pivot + UI Panel look at player
  (Transformation|SetWorldRotation _uipivot (Math|Rotator|FindLookatRotation (Transformation|GetWorldLocation _uipivot) (Transformation|GetActorLocation (Game|Player|GetPlayerPawn 0))) false false)
  (Transformation|SetWorldRotation _quizui (Math|Rotator|FindLookatRotation (Transformation|GetWorldLocation _quizui) (Transformation|GetActorLocation (Game|Player|GetPlayerPawn 0))) false false))

(fn ConstructionScript)

(fn PopulateQuiz
  (bind _aswbp_planet_quiz_ui (Utilities|Casting|CastToWBP_PlanetQuizUI (UserInterface|GetUserWidgetObject (Variables|Default|GetQuizUI))))
  (Variables|Default|SetQuizWidget _aswbp_planet_quiz_ui)
  (bind _returnvalue (Utilities|GetDataTableRow "/Game/Data/DT_Quiz.DT_Quiz" (Utilities|String|StringToName (Variables|Default|GetPlanetType)))
    (:then
      (Variables|/Script/UMG.MultiLineEditableText|SetText (Variables|/Game/UI/WBP_PlanetQuizUI.WBP_PlanetQuizUI_C|GetQuestionText _aswbp_planet_quiz_ui) (.question _returnvalue))
      (Default|ConstructAnswerButtonArray (Variables|Default|GetQuizWidget))
      (Default|ConstructAnswerButtonTextArray (Variables|Default|GetQuizWidget))
      (for (_array_element _array_index) (Variables|/Game/UI/WBP_PlanetQuizUI.WBP_PlanetQuizUI_C|GetAnswerButtonTextBoxes (Variables|Default|GetQuizWidget))
        (Rendering|Components|TextRender|SetText _array_element (Utilities|Array|Get(acopy) (.answers _returnvalue) _array_index))))))

(fn UpdateButtonSelection
  (params (SelectedButtonIndex :type Integer))
  (Default|UpdateButtonSelection (Variables|Default|GetQuizWidget) SelectedButtonIndex))

(fn ToggleQuizUIVisibility
  (params (bIsVisible :type Boolean))
  (Rendering|SetVisibility (Variables|Default|GetQuizUI) bIsVisible true))