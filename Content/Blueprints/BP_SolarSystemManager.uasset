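; BP_SolarSystemManager tracks which planets are unlocked and checks for the game's win condition.
; UnlockPlanet marks a planet true in the UnlockedPlanets map, then calls AreAllPlanetsUnlocked, which loops over the map's values to test whether all are set.
; The outcome only prints a won or not-won debug string, and the event graph and construction script are empty.
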(event EventBeginPlay)

(event Collision|EventActorBeginOverlap
  (params (OtherActor :type Actor%20Object%20Reference)))

(event EventTick
  (params (DeltaSeconds :type Float%20%28single-precision%29)))

(fn ConstructionScript)

(fn AreAllPlanetsUnlocked
  (bind _bresult (LocalVariables|GetbResult))
  (bind _valuepin (Utilities|Map|ForEachLoop(Map) (Variables|Default|GetUnlockedPlanets))
    (:then
      (LocalVariables|SetbAreAllUnlocked (and _valuepin _bresult)))
    (:CompletedPin
      (return _bresult))))

(fn UnlockPlanet
  (params (Planet :type String))
  (Utilities|Map|Add (Variables|Default|GetUnlockedPlanets) Planet true)
  (bind _bresult (CallFunction|AreAllPlanetsUnlocked))
  (if _bresult
    (Development|PrintString "GAME WON GAME WON")
    (else
      (Development|PrintString "STILL A LOSER"))))